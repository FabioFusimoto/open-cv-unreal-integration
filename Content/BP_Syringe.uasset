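; BP_Syringe is a syringe actor whose world pose is set from JSON data.
; SetPositionFromResponse reads roll, pitch, yaw and x, y, z from a named nested JSON object and applies them to the root component without sweeping.
; Overlap begin and end events print brief debug messages when the other actor's display name is "Arm".
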(event EventBeginPlay)

(event Collision|EventActorBeginOverlap
  (params (OtherActor :type Actor%20Object%20Reference))
  (if (Utilities|Enum|Equal(Enum) (Utilities|GetDisplayName OtherActor) "Arm")
    (Development|PrintString "Overlap Started: Arm" true true "(R=0.405760,G=0.000000,B=1.000000,A=1.000000)" 0.5)))

(event Collision|EventActorEndOverlap
  (params (OtherActor :type Actor%20Object%20Reference))
  (if (Utilities|Enum|Equal(Enum) (Utilities|GetDisplayName OtherActor) "Arm")
    (Development|PrintString "Overlap Ended: Arm" true true "(R=0.405760,G=0.000000,B=1.000000,A=1.000000)" 0.5)))

(fn ConstructionScript)

(fn SetPositionfromResponse
  (params (JSON :type Va%20Rest%20Json%20Object%20Object%20Reference) (FieldName :type String))
  (bind _returnvalue (Class|VaRestJsonObject|GetObjectField JSON FieldName))
  (Transformation|SetWorldRotation (Variables|Default|GetDefaultSceneRoot) (Math|Rotator|MakeRotator (Class|VaRestJsonObject|GetNumberField _returnvalue "0_roll") (Class|VaRestJsonObject|GetNumberField _returnvalue "1_pitch") (Class|VaRestJsonObject|GetNumberField _returnvalue "2_yaw")) false false)
  (Transformation|SetWorldLocation (Variables|Default|GetDefaultSceneRoot) (Math|Vector|MakeVector (Class|VaRestJsonObject|GetNumberField _returnvalue "3_x") (Class|VaRestJsonObject|GetNumberField _returnvalue "4_y") (Class|VaRestJsonObject|GetNumberField _returnvalue "5_z")) false false))