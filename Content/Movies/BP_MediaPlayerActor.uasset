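; Actor that opens a video file in a media player on BeginPlay, with the file chosen through external configuration.
; A named command-line option supplies the path of a configuration text file, which is read as a comma-separated list of video paths.
; The entry at VideoIndex has its backslashes converted to forward slashes before opening.
; A missing option or failed open prints an on-screen error.
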(event EventBeginPlay
  (CallFunction|SetConfigurationFilePath)
  (CallFunction|SetVideoPath)
  (CallFunction|OpenVideoFile))

(fn ConstructionScript)

(fn ContainsCommandLineOption
  (params (Option :type String))
  (bind _returnvalue (Utilities|GetCommandLine))
  (for _array_element (Utilities|String|ParseIntoArray _returnvalue " ")
    (if (Utilities|String|Contains _array_element Option)
      (return true)))
  (return false))

(fn GetCommandLineOption
  (params (Option :type String))
  (bind _returnvalue (Utilities|GetCommandLine))
  (for _array_element (Utilities|String|ParseIntoArray _returnvalue " ")
    (if (Utilities|String|Contains _array_element Option)
      (return (.RightS (Utilities|String|Split _array_element "="))))))

(fn SetConfigurationFilePath
  (bind _commandlineoption (Variables|Default|GetCommandLineOption))
  (bind _contains (CallFunction|ContainsCommandLineOption _commandlineoption))
  (if _contains
    (bind _value (CallFunction|GetCommandLineOption _commandlineoption))
    (Variables|Default|SetConfigurationFilePath _value)
    (else
      (Development|PrintString (Utilities|String|Append "No option " _commandlineoption) true true "(R=1.000000,G=0.011645,B=0.000000,A=1.000000)" 1e+02))))

(fn SetVideoPath
  (bind _result (Class|VictoryBPFunctionLibrary|LoadStringfromFile (Variables|Default|GetConfigurationFilePath)))
  (Variables|Default|SetVideoPath (Utilities|Array|Get(acopy) (Utilities|String|ParseIntoArray _result ",") (Variables|Default|GetVideoIndex))))

(fn OpenVideoFile
  (bind _videopath (Variables|Default|GetVideoPath))
  (bind _returnvalue (Utilities|String|Replace _videopath "\\" "/"))
  (bind _returnvalue_2 (Class|MediaPlayer|OpenFile (Variables|Default|GetMediaPlayer) _returnvalue))
  (if (not _returnvalue_2)
    (Development|PrintString (Utilities|String|Append "Error when opening: " _returnvalue) true true "(R=1.000000,G=0.000000,B=0.000000,A=1.000000)" 1e+02)))