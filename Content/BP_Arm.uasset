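; BP_Arm is an actor whose Arm and Marker1 components are posed from JSON data.
; SetPositionFromResponse reads roll, pitch, yaw and X, Y, Z numbers from the named object field of the passed JSON.
; It applies the same values to Arm and then Marker1, setting rotation in relative space but location in world space, without sweep.
; The event graph and construction script are empty.
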(event EventBeginPlay)

(event Collision|EventActorBeginOverlap
  (params (OtherActor :type Actor%20Object%20Reference)))

(event EventTick
  (params (DeltaSeconds :type Float%20%28single-precision%29)))

(fn ConstructionScript)

(fn SetPositionfromResponse
  (params (JSON :type Va%20Rest%20Json%20Object%20Object%20Reference) (FieldName :type String))
  (bind _returnvalue (Class|VaRestJsonObject|GetObjectField JSON FieldName))
  (bind _returnvalue_2 (Class|VaRestJsonObject|GetNumberField _returnvalue "0_roll"))
  (bind _returnvalue_3 (Class|VaRestJsonObject|GetNumberField _returnvalue "1_pitch"))
  (bind _returnvalue_4 (Class|VaRestJsonObject|GetNumberField _returnvalue "2_yaw"))
  (bind _returnvalue_5 (Class|VaRestJsonObject|GetNumberField _returnvalue "3_x"))
  (bind _returnvalue_6 (Class|VaRestJsonObject|GetNumberField _returnvalue "4_y"))
  (bind _returnvalue_7 (Class|VaRestJsonObject|GetNumberField _returnvalue "5_z"))
  (bind _returnvalue_8 (Math|Rotator|MakeRotator _returnvalue_2 _returnvalue_3 _returnvalue_4))
  (bind _returnvalue_9 (Math|Vector|MakeVector _returnvalue_5 _returnvalue_6 _returnvalue_7))
  (Utilities|FlowControl|Sequence
    (:then_0
      (Transformation|SetRelativeRotation (Variables|Default|GetArm) _returnvalue_8 false false)
      (Transformation|SetWorldLocation (Variables|Default|GetArm) _returnvalue_9 false false))
    (:then_1
      (Transformation|SetRelativeRotation (Variables|Default|GetMarker_1) _returnvalue_8 false false)
      (Transformation|SetWorldLocation (Variables|Default|GetMarker_1) _returnvalue_9 false false))))