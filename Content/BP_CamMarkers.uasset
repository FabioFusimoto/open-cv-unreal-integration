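; BP_CamMarkers is a camera-marker Blueprint that places mesh components from JSON response data and prints a marker's transform for debugging.
; SetPositionFromResponse reads a named JSON object and applies its roll/pitch/yaw as relative rotation and its XYZ as world location, mixing coordinate spaces.
; PrintMarkersPosition prints only Marker0's world location and rotation on screen.
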(fn ConstructionScript)

(fn PrintMarkersPosition
  (bind _duration (Variables|Default|GetDuration))
  (Utilities|FlowControl|Sequence
    (:then_0
      (Development|PrintString (Utilities|String|ToString(Vector) (Transformation|GetWorldLocation (Variables|Default|GetMarker_0))) true true "(R=1.000000,G=0.000000,B=0.689732,A=1.000000)" _duration))
    (:then_1
      (Development|PrintString (Utilities|String|ToString(Rotator) (Transformation|GetWorldRotation (Variables|Default|GetMarker_0))) true true "(R=1.000000,G=0.000000,B=0.689732,A=1.000000)" _duration))))

(fn SetPositionfromResponse
  (params (Mesh :type Scene%20Component%20Object%20Reference) (JSON :type Va%20Rest%20Json%20Object%20Object%20Reference) (FieldName :type String))
  (bind _returnvalue (Class|VaRestJsonObject|GetObjectField JSON FieldName))
  (Transformation|SetRelativeRotation Mesh (Math|Rotator|MakeRotator (Class|VaRestJsonObject|GetNumberField _returnvalue "0_roll") (Class|VaRestJsonObject|GetNumberField _returnvalue "1_pitch") (Class|VaRestJsonObject|GetNumberField _returnvalue "2_yaw")) false false)
  (Transformation|SetWorldLocation Mesh (Math|Vector|MakeVector (Class|VaRestJsonObject|GetNumberField _returnvalue "3_x") (Class|VaRestJsonObject|GetNumberField _returnvalue "4_y") (Class|VaRestJsonObject|GetNumberField _returnvalue "5_z")) false false))