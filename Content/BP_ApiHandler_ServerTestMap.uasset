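; Test-map API handler that drives a camera and a syringe from poses served by a local HTTP tracking server.
; BeginPlay sets Leap Motion to VR mode and requests pivot loading; the callback marks the session loaded.
; Tick then requests multi-pivot poses every frame without throttling, and the JSON response positions both objects and stores the target pivot ID.
; The timer for printing that ID is unconnected.
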(event Custom|PoseResponse
  (params (Request :type Va%20Rest%20Request%20JSON%20Object%20Reference))
  (if (Variables|Default|GetSessionLoaded)
    (bind _returnvalue (Class|VaRestRequestJSON|GetResponseObject Request))
    (Utilities|FlowControl|Sequence
      (:then_0
        (Default|SetPositionfromResponse (Variables|Default|GetCamera) _returnvalue "hmd"))
      (:then_1
        (Default|SetPositionfromResponse (Variables|Default|GetSyringe) _returnvalue "syringe_102"))
      (:then_2
        (Variables|Default|SetTargetPivotId (Class|VaRestJsonObject|GetStringField _returnvalue "target_pivot_id"))))
    (else
      (Development|PrintString "Session not loaded!" true true "(R=0.548188,G=0.000000,B=1.000000,A=1.000000)" 0.5))))

(event Custom|PivotLoaded
  (params (Request :type Va%20Rest%20Request%20JSON%20Object%20Reference))
  (Variables|Default|SetSessionLoaded true))

(event EventBeginPlay
  (Class|LeapBlueprintFunctionLibrary|SetLeapMode "LEAP_MODE_VR" "LEAP_SMOOTH")
  (Class|VaRestLibrary|CallURL "http://127.0.0.1:5000/load-pivots" "GET" "json" 0 (delegate Custom|PivotLoaded)))

(event EventTick
  (params (DeltaSeconds :type Float%20%28single-precision%29))
  (if (Variables|Default|GetSessionLoaded)
    (Class|VaRestLibrary|CallURL "http://127.0.0.1:5000/pose-from-multiple-pivots?reference=9&context=test&pivot_to_save=" "GET" "json" (Class|VaRestJsonObject|ConstructJsonObject) (delegate Custom|PoseResponse))))

(fn ConstructionScript)

(fn PrintDebug
  (Development|PrintString (Utilities|String|Append "Target pivot id: " (Variables|Default|GetTargetPivotId)) true true "(R=0.000000,G=0.660000,B=1.000000,A=1.000000)" (Variables|Default|GetDuration)))